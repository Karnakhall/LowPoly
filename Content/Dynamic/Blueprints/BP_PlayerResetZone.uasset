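; BP_PlayerResetZone is a trigger volume that returns the player character to the last saved checkpoint on overlap.
; It loads the "checksave" save slot, zeroes the character's velocity, then restores location, rotation, collected keys and mana.
; It then calls ChecpointLoadstuff on My_gamestate to finish the checkpoint reload.
; The construction script sets the Box transform from the Height and Size variables.
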(event `self.Box.OnComponentBeginOverlap`
  (params (OverlappedComponent :type "PrimitiveComponent Object Reference") (OtherActor :type "Actor Object Reference") (OtherComp :type "PrimitiveComponent Object Reference") (OtherBodyIndex :type Integer) (bFromSweep :type Boolean) (SweepResult :type "HitResult Structure (by ref)"))
  (bind _asbp_player_character (cast `/Game/Dynamic/Blueprints/CHaracterMovement/BP_PlayerCharacter` OtherActor))
  (bind _returnvalue (`GameplayStatics.LoadGameFromSlot` "checksave"))
  (bind _assave_game_obj (cast `/Game/Dynamic/Blueprints/checkpoints/Save_Game_OBJ` _returnvalue))
  (`Character.LaunchCharacter` _asbp_player_character (0.0 0.0 0.0) true true)
  (`self.K2_SetActorLocation` _asbp_player_character (`/Game/Dynamic/Blueprints/checkpoints/Save_Game_OBJ.PlayerLoc` _assave_game_obj) false false)
  (`self.K2_SetActorRotation` _asbp_player_character (`KismetMathLibrary.Conv_VectorToRotator` (`/Game/Dynamic/Blueprints/checkpoints/Save_Game_OBJ.PlayerRot` _assave_game_obj)) false)
  (set `/Game/Dynamic/Blueprints/CHaracterMovement/BP_PlayerCharacter.KeysCollected` (`KismetMathLibrary.Conv_IntToByte` (`/Game/Dynamic/Blueprints/checkpoints/Save_Game_OBJ.Ammountofkeyscollected` _assave_game_obj)) _asbp_player_character)
  (bind _asbp_player_character_2 (cast `/Game/Dynamic/Blueprints/CHaracterMovement/BP_PlayerCharacter` (`GameplayStatics.GetPlayerCharacter` 0)))
  (set `/Game/Dynamic/Blueprints/CHaracterMovement/BP_PlayerCharacter.ManaPoints` (`/Game/Dynamic/Blueprints/checkpoints/Save_Game_OBJ.manasave` _assave_game_obj) _asbp_player_character_2)
  (bind _asmy_gamestate (cast `/Game/Dynamic/Blueprints/checkpoints/My_gamestate` (`GameplayStatics.GetGameState`)))
  (`/Game/Dynamic/Blueprints/checkpoints/My_gamestate.ChecpointLoadstuff` _asmy_gamestate))

(fn `UserConstructionScript`
  (bind _size (`self.Size`))
  (`SceneComponent.K2_SetWorldTransform` (`self.Box`) (`KismetMathLibrary.MakeTransform` (`KismetMathLibrary.MakeVector` 0.0 0.0 (`self.Height`)) (struct) (`KismetMathLibrary.MakeVector` _size _size 1.0)) false false))