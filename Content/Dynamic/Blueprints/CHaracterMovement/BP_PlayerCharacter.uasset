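; BP_PlayerCharacter is the player character, handling interaction, HUD, pause and win menus, and saving.
; Interaction keys drive ACInteractionTrace, while left click also messages an overlapping BI_Interaction actor.
; BeginPlay builds widgets, writes the start location to the "checksave" slot and starts a recurring grounded-location record.
; Hit starts a delayed, endless loop spawning and triggering FS_MasterField at the hit point; EventGameOver is empty.
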(event `EventWinGame`
  (bind _returnvalue (`GameplayStatics.GetPlayerController` 0))
  (bind _endmenu (`self.EndMenu`))
  ;[1 1 1] Win Game
  (`WidgetLayoutLibrary.RemoveAllWidgets`)
  (`UserWidget.AddToViewport` _endmenu 0)
  (`WidgetBlueprintLibrary.SetInputMode_UIOnlyEx` _returnvalue _endmenu)
  (set `PlayerController.bShowMouseCursor` true _returnvalue)
  (`GameplayStatics.SetGamePaused` true))

(event `EventGameOver`
  ;[1 1 1] Game Over
)

(event `InputAction|Switch Camera`
  (params (Key :type "Key Structure"))
  ;[1 1 1] Switch Camera
)

(event `SavePlayerLocation`
  ;[1 1 1] Save Player Location  (disabled) (checpoint are on)
  (if (not (`NavMovementComponent.IsFalling` (`self.CharacterMovement`)))
    (set `self.SaveLocation` (`self.K2_GetActorLocation`)))
  (`KismetSystemLibrary.Delay` 2.0)
  (`self.SavePlayerLocation`))

(event `Key|F`
  (params (Key :type "Key Structure"))
  (bind _ac_interactiontrace (`self.AC_InteractionTrace`))
  (:`Pressed`
    (`/Game/Dynamic/Interactions/AC_InteractionTrace.TryToInteract` _ac_interactiontrace true))
  (:`Released`
    (`/Game/Dynamic/Interactions/AC_InteractionTrace.TryToInteract` _ac_interactiontrace false)))

(event `Key|E`
  (params (Key :type "Key Structure"))
  (bind _ac_interactiontrace (`self.AC_InteractionTrace`))
  (:`Pressed`
    (`/Game/Dynamic/Interactions/AC_InteractionTrace.TryToInteract` _ac_interactiontrace true))
  (:`Released`
    (`/Game/Dynamic/Interactions/AC_InteractionTrace.TryToInteract` _ac_interactiontrace false)))

(event `Key|Q`
  (params (Key :type "Key Structure"))
  (bind _ac_interactiontrace (`self.AC_InteractionTrace`))
  (:`Pressed`
    (`/Game/Dynamic/Interactions/AC_InteractionTrace.TryToInteract` _ac_interactiontrace true))
  (:`Released`
    (`/Game/Dynamic/Interactions/AC_InteractionTrace.TryToInteract` _ac_interactiontrace false)))

(event `Key|LeftMouseButton`
  (params (Key :type "Key Structure"))
  (bind _ac_interactiontrace (`self.AC_InteractionTrace`))
  (:`Pressed`
    (`/Game/Dynamic/Interactions/AC_InteractionTrace.TryToInteract` _ac_interactiontrace true))
  (:`Released`
    (`/Game/Dynamic/Interactions/AC_InteractionTrace.TryToInteract` _ac_interactiontrace false)))

(event `Key|LeftMouseButton`
  (params (Key :type "Key Structure"))
  (:`Pressed`
    (for _array_element (`self.GetOverlappingActors` "/Script/Engine.Actor")
      (if (`KismetSystemLibrary.DoesImplementInterface` _array_element "/Game/Dynamic/Interactions/BI_Interaction.BI_Interaction_C")
        (message `/Game/Dynamic/Interactions/BI_Interaction.Interact` _array_element)
        (break)))))

(event `self.ReceiveBeginPlay`
  (bind _returnvalue (`self.K2_GetActorLocation`))
  (`|ExecutionSequence`
    (:`then_0`
      (bind _returnvalue_2 (`|CreateWidget` "/Game/Dynamic/Blueprints/UserInterface/WB_ManaPoints.WB_ManaPoints_C"))
      (`UserWidget.AddToViewport` _returnvalue_2 0))
    (:`then_1`
      (bind _returnvalue_3 (`|CreateWidget` "/Game/Dynamic/Interactions/WB_MyHud.WB_MyHud_C"))
      (bind _output_get (set `self.MyHud` _returnvalue_3))
      (`UserWidget.AddToViewport` _output_get 0)
      (`self.SavePlayerLocation`)
      (`self.SetupInteractionTrace`)
      (bind _returnvalue_4 (`|CreateWidget` "/Game/Menu/WII_EndMenu.WII_EndMenu_C"))
      (set `self.EndMenu` _returnvalue_4)
      (`WidgetBlueprintLibrary.SetInputMode_GameOnly` (`GameplayStatics.GetPlayerController` 0)))
    (:`then_2`
      ;[1 1 1] Saving location of player also a base for saves
      (bind _returnvalue_5 (`GameplayStatics.DoesSaveGameExist` "checksave"))
      (if _returnvalue_5
        (bind _returnvalue_6 (`GameplayStatics.LoadGameFromSlot` "checksave"))
        (bind _assave_game_obj (cast `/Game/Dynamic/Blueprints/checkpoints/Save_Game_OBJ` _returnvalue_6))
        (set `/Game/Dynamic/Blueprints/checkpoints/Save_Game_OBJ.PlayerLoc` _returnvalue _assave_game_obj)
        (`GameplayStatics.SaveGameToSlot` _assave_game_obj "checksave")
        (else
          (bind _returnvalue_7 (`GameplayStatics.CreateSaveGameObject` "/Game/Dynamic/Blueprints/checkpoints/Save_Game_OBJ.Save_Game_OBJ_C"))
          (set `/Game/Dynamic/Blueprints/checkpoints/Save_Game_OBJ.PlayerLoc` _returnvalue _returnvalue_7)
          (`GameplayStatics.SaveGameToSlot` _returnvalue_7 "checksave"))))))

(event `InputAction|Pause` :paused true
  (params (Key :type "Key Structure"))
  (bind _returnvalue (`GameplayStatics.GetPlayerController` 0))
  (bind _returnvalue_2 (`GameplayStatics.GetPlayerController` 0))
  ;[1 1 1] Pause Menu
  (:`Pressed`
    (if (`GameplayStatics.IsGamePaused`)
      (`Widget.RemoveFromParent` (stale _returnvalue_3))
      (`WidgetBlueprintLibrary.SetInputMode_GameOnly` _returnvalue_2)
      (set `PlayerController.bShowMouseCursor` false _returnvalue_2)
      (`GameplayStatics.SetGamePaused` false)
      (else
        (bind _returnvalue_3 (`|CreateWidget` "/Game/Menu/WII_PauseMenu.WII_PauseMenu_C"))
        (`UserWidget.AddToViewport` _returnvalue_3 0)
        (`GameplayStatics.SetGamePaused` true)
        (`WidgetBlueprintLibrary.SetInputMode_GameAndUIEx` _returnvalue null)
        (set `PlayerController.bShowMouseCursor` true _returnvalue)))))

(event `self.ReceiveHit`
  (params (MyComp :type "PrimitiveComponent Object Reference") (Other :type "Actor Object Reference") (OtherComp :type "PrimitiveComponent Object Reference") (bSelfMoved :type Boolean) (HitLocation :type "Vector Structure") (HitNormal :type "Vector Structure") (NormalImpulse :type "Vector Structure") (Hit :type "HitResult Structure (by ref)"))
  (`KismetSystemLibrary.Delay` 1.5 :!label _label)
  (bind _returnvalue (`|SpawnActorFromClass` "/Game/Dynamic/Interactions/FS_MasterField.FS_MasterField_C" (`KismetMathLibrary.MakeTransform` HitLocation) "Undefined" "MultiplyWithRoot" null null))
  (set `/Game/Dynamic/Interactions/FS_MasterField.ActivationType` "NewEnumerator4" _returnvalue)
  (`/Game/Dynamic/Interactions/FS_MasterField.CE_Trigger` _returnvalue)
  (goto _label))

(fn `SetupInteractionTrace`
  (if (`self.IsLocallyControlled`)
    (`ActorComponent.SetComponentTickEnabled` (`self.AC_InteractionTrace`) true)))

(fn `UserConstructionScript`)