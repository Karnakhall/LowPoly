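; Portal actor that the player can open once they have pushed a Key Stone and collected enough keys.
; On overlap it checks the player character's progress, sets its screen message, and enables input only when both requirements are met.
; UseObject then reveals the portal's Niagara effect and light, with no teleport logic here.
; Leaving clears the message and disables input; interaction events are empty, and the unlock-flag and rotation timeline logic is disconnected.
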(event `InputAction|UseObject`
  (params (Key :type "Key Structure"))
  (:`Pressed`
    (`SceneComponent.SetVisibility` (`self.PortalNiagara`) true false)
    (`SceneComponent.SetVisibility` (`self.PortalLight`) true false)))

(event `self.PortalCollision.OnComponentBeginOverlap`
  (params (OverlappedComponent :type "PrimitiveComponent Object Reference") (OtherActor :type "Actor Object Reference") (OtherComp :type "PrimitiveComponent Object Reference") (OtherBodyIndex :type Integer) (bFromSweep :type Boolean) (SweepResult :type "HitResult Structure (by ref)"))
  (bind _asbp_player_character (cast `/Game/Dynamic/Blueprints/CHaracterMovement/BP_PlayerCharacter` OtherActor))
  (if (and (>= (`/Game/Dynamic/Blueprints/CHaracterMovement/BP_PlayerCharacter.KeyStonePushed` _asbp_player_character) 1) (>= (`/Game/Dynamic/Blueprints/CHaracterMovement/BP_PlayerCharacter.KeysCollected` _asbp_player_character) 2))
    (set `/Game/Dynamic/Blueprints/CHaracterMovement/BP_PlayerCharacter.ScreenMessage` "Press F to open portal" _asbp_player_character)
    (`self.EnableInput` (`GameplayStatics.GetPlayerController` 0))
    (else
      (set `/Game/Dynamic/Blueprints/CHaracterMovement/BP_PlayerCharacter.ScreenMessage` "You must move Key Stone and pick up all keys to open portal" _asbp_player_character))))

(event `self.PortalCollision.OnComponentEndOverlap`
  (params (OverlappedComponent :type "PrimitiveComponent Object Reference") (OtherActor :type "Actor Object Reference") (OtherComp :type "PrimitiveComponent Object Reference") (OtherBodyIndex :type Integer))
  (bind _asbp_player_character (cast `/Game/Dynamic/Blueprints/CHaracterMovement/BP_PlayerCharacter` OtherActor))
  (set `/Game/Dynamic/Blueprints/CHaracterMovement/BP_PlayerCharacter.ScreenMessage` "" _asbp_player_character)
  (`self.DisableInput` (`GameplayStatics.GetPlayerController` 0)))

(event `/Game/Dynamic/Interactions/BI_Interaction.Interact`)

(event `/Game/Dynamic/Interactions/BI_Portal.PickUpKey`)

(fn `GetInteractionWidgetRef`
  (returns (Ref :type "WidgetComponent Object Reference"))
  (return null))

(fn `UserConstructionScript`)