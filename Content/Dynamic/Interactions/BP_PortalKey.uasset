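; BP_PortalKey is a collectible key that increments the player character's KeysCollected on overlap, then destroys itself.
; A separate Interact event sends PickUpKeyMessage to its Portal and also destroys the key.
; Interface events toggle the cube's custom-depth on focus and flip InteractToggle through InteractOnServer.
; OnRep_InteractToggle is empty in effect, as its point light visibility logic is disconnected.
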(event `/Game/Dynamic/Interactions/BI_Interaction.Interact`
  (message `/Game/Dynamic/Interactions/BI_Portal.PickUpKey` (`self.Portal`))
  (`self.K2_DestroyActor`))

(event `self.Interface_ToggleFocus`
  (params (Focus :type Boolean))
  (`PrimitiveComponent.SetRenderCustomDepth` (`self.Cube`) Focus))

(event `self.ReceiveActorBeginOverlap`
  (params (OtherActor :type "Actor Object Reference"))
  (bind _asbp_player_character (cast `/Game/Dynamic/Blueprints/CHaracterMovement/BP_PlayerCharacter` OtherActor))
  (set `/Game/Dynamic/Blueprints/CHaracterMovement/BP_PlayerCharacter.KeysCollected` (+ (`/Game/Dynamic/Blueprints/CHaracterMovement/BP_PlayerCharacter.KeysCollected` _asbp_player_character) 1) _asbp_player_character)
  (`self.K2_DestroyActor`))

(event `self.InterfaceInteract`
  (`self.InteractOnServer`))

(event `InteractOnServer`
  (set `self.InteractToggle` (not (`self.InteractToggle`))))

(fn `GetInteractionWidgetRef`
  (returns (Ref :type "WidgetComponent Object Reference"))
  (return (`self.Widget`)))

(fn `OnRep_InteractToggle`
  ;[1 1 1] Visibility of Point light
)

(fn `UserConstructionScript`)