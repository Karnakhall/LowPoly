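; BP_TestInteractionActor is a test interactable that outlines on focus, toggles on interact and rotates through player input.
; The interaction interface drives the cube's custom depth, supplies its widget and calls InteractOnServer to flip InteractToggle, whose OnRep point-light logic is disconnected.
; BlocksCollision enables input while a BP_PlayerCharacter overlaps, letting RotateBlocks play a timeline that offsets actor yaw from its starting rotation.
; Releasing the input resets the timeline's time.
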(event `/Game/Dynamic/Interactions/BI_Interaction.Interface_ToggleFocus`
  (params (Focus :type Boolean))
  (`PrimitiveComponent.SetRenderCustomDepth` (`self.Cube`) Focus))

(event `/Game/Dynamic/Interactions/BI_Interaction.InterfaceInteract`
  (`self.InteractOnServer`))

(event `InteractOnServer`
  (set `self.InteractToggle` (not (`self.InteractToggle`))))

(event `InputAction|RotateBlocks`
  (params (Key :type "Key Structure"))
  ;[1 1 1] RotateBlocks
  (:`Pressed`
    (bind _output_get (set `self.InitialBlocksRotation` (`self.K2_GetActorRotation`)))
    (bind (_direction _rotateblocksmovement) (`Timeline|RotateBlocks Timeline` :!label _label)
      (:`Update`
        (`self.K2_SetActorRotation` (`KismetMathLibrary.MakeRotator` (.roll _output_get) (.pitch _output_get) (- (.yaw _output_get) _rotateblocksmovement))))))
  (:`Released`
    (goto _label :!via `SetNewTime`)))

(event `self.BlocksCollision.OnComponentBeginOverlap`
  (params (OverlappedComponent :type "PrimitiveComponent Object Reference") (OtherActor :type "Actor Object Reference") (OtherComp :type "PrimitiveComponent Object Reference") (OtherBodyIndex :type Integer) (bFromSweep :type Boolean) (SweepResult :type "HitResult Structure (by ref)"))
  ;[1 1 1] enable/disable rotateblocks
  (cast `/Game/Dynamic/Blueprints/CHaracterMovement/BP_PlayerCharacter` OtherActor)
  (`self.EnableInput` (`GameplayStatics.GetPlayerController` 0)))

(event `self.BlocksCollision.OnComponentEndOverlap`
  (params (OverlappedComponent :type "PrimitiveComponent Object Reference") (OtherActor :type "Actor Object Reference") (OtherComp :type "PrimitiveComponent Object Reference") (OtherBodyIndex :type Integer))
  ;[1 1 1] enable/disable rotateblocks
  (cast `/Game/Dynamic/Blueprints/CHaracterMovement/BP_PlayerCharacter` OtherActor)
  (`self.DisableInput` (`GameplayStatics.GetPlayerController` 0)))

(fn `GetInteractionWidgetRef`
  (returns (Ref :type "WidgetComponent Object Reference"))
  (return (`self.Widget`)))

(fn `OnRep_InteractToggle`
  ;[1 1 1] Visibility of Point light
)

(fn `UserConstructionScript`)