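; BP_ManaRefill_FireArch is a single-use mana refill interactable that grants mana points when its trigger box is overlapped.
; The first overlap by any actor adds ManaValue to player 0's BP_PlayerCharacter, without checking that the overlapping actor is that player.
; It then spawns an active Niagara effect, removes the static one after a short delay and sets the point light's intensity, with debug prints along the way.
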(event `self.ReceiveActorBeginOverlap`
  (params (OtherActor :type "Actor Object Reference")))

(event `self.Box.OnComponentBeginOverlap`
  (params (OverlappedComponent :type "PrimitiveComponent Object Reference") (OtherActor :type "Actor Object Reference") (OtherComp :type "PrimitiveComponent Object Reference") (OtherBodyIndex :type Integer) (bFromSweep :type Boolean) (SweepResult :type "HitResult Structure (by ref)"))
  (bind _manavalue (`self.ManaValue`))
  (`/Engine/EditorBlueprintResources/StandardMacros.DoOnce` false
    (:`Completed`
      (`KismetSystemLibrary.PrintString` (`KismetStringLibrary.Concat_StrStr` (`KismetSystemLibrary.GetDisplayName` OtherActor) " overlapped "))
      (bind _asbp_player_character (cast `/Game/Dynamic/Blueprints/CHaracterMovement/BP_PlayerCharacter` (`GameplayStatics.GetPlayerCharacter` 0)))
      (set `/Game/Dynamic/Blueprints/CHaracterMovement/BP_PlayerCharacter.ManaPoints` (+ (`/Game/Dynamic/Blueprints/CHaracterMovement/BP_PlayerCharacter.ManaPoints` _asbp_player_character) _manavalue) _asbp_player_character)
      (`KismetSystemLibrary.PrintString` (`KismetStringLibrary.Concat_StrStr` (`KismetStringLibrary.Conv_IntToString` _manavalue) " mana points added"))
      (`NiagaraFunctionLibrary.SpawnSystemAtLocation` "/Game/Graphics/VFX/FX_Mana/NS_ManaActive.NS_ManaActive" (`self.K2_GetActorLocation`))
      (`KismetSystemLibrary.Delay` 0.7)
      (`ActorComponent.K2_DestroyComponent` (`self.NS_Mana_Static`))
      (`KismetSystemLibrary.Delay` 0.45)
      (`LightComponent.SetIntensity` (`self.PointLight`) 500.0))))

(fn `UserConstructionScript`)