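; Interactable block actor that pitches on a timeline two seconds after a player character begins overlapping it.
; Interface focus toggles a custom-depth highlight on the cube.
; Interacting calls a server event that flips InteractToggle, but its OnRep light-visibility logic is disconnected, so it does not affect rotation or lighting.
; Functions to check and deduct the player's mana cost exist but are never called here.
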(event `self.ReceiveActorBeginOverlap`
  (params (OtherActor :type "Actor Object Reference"))
  (cast `/Game/Dynamic/Blueprints/CHaracterMovement/BP_PlayerCharacter` OtherActor)
  (if true
    (`KismetSystemLibrary.Delay` 2.0)
    (bind (_direction _rotateblock) (`Timeline|Rotate Block` :!via `PlayFromStart`)
      (:`Update`
        (`self.K2_SetActorRotation` (`KismetMathLibrary.MakeRotator` 0.0 _rotateblock))))))

(event `self.Interface_ToggleFocus`
  (params (Focus :type Boolean))
  (`PrimitiveComponent.SetRenderCustomDepth` (`self.Cube`) Focus))

(event `self.InterfaceInteract`
  (`self.InteractOnServer`))

(event `InteractOnServer`
  (set `self.InteractToggle` (not (`self.InteractToggle`))))

(event `OnActorBeginOverlap_Event` :!signature `self.OnActorBeginOverlap`
  (params (OverlappedActor :type "Actor Object Reference") (OtherActor :type "Actor Object Reference")))

(fn `FnIsEnoughMana`
  (bind _asbp_player_character (cast `/Game/Dynamic/Blueprints/CHaracterMovement/BP_PlayerCharacter` (`GameplayStatics.GetPlayerCharacter` 0)))
  (if (>= (- (`/Game/Dynamic/Blueprints/CHaracterMovement/BP_PlayerCharacter.ManaPoints` _asbp_player_character) (`self.ManaCostToRotate`)) 0)
    (set `self.EnoughMana` true))
  (return))

(fn `FnManaSubtractingAndReset`
  (bind _asbp_player_character (cast `/Game/Dynamic/Blueprints/CHaracterMovement/BP_PlayerCharacter` (`GameplayStatics.GetPlayerCharacter` 0)))
  (set `/Game/Dynamic/Blueprints/CHaracterMovement/BP_PlayerCharacter.ManaPoints` (- (`/Game/Dynamic/Blueprints/CHaracterMovement/BP_PlayerCharacter.ManaPoints` _asbp_player_character) (`self.ManaCostToRotate`)) _asbp_player_character)
  (set `self.EnoughMana` false)
  (return))

(fn `GetInteractionWidgetRef`
  (returns (Ref :type "WidgetComponent Object Reference"))
  (return null))

(fn `OnRep_InteractToggle`
  ;[1 1 1] Visibility of Point light
)

(fn `UserConstructionScript`)