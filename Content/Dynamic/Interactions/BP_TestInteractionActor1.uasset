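; Test interactable actor that the player rotates in yaw with left or right mouse clicks, spending mana per turn.
; Overlapping BlocksCollision enables input; each click checks and deducts player mana, then runs a timeline guarded by DoOnce and IsRotating, with left clicks also spawning effects every update.
; Interface events toggle custom-depth highlighting and set replicated InteractToggle, but its OnRep point-light logic is disconnected.
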(event `self.Interface_ToggleFocus`
  (params (Focus :type Boolean))
  (`PrimitiveComponent.SetRenderCustomDepth` (`self.Cube`) Focus))

(event `self.InterfaceInteract`
  (`self.InteractOnServer`))

(event `InteractOnServer`
  (set `self.InteractToggle` (not false)))

(event `Key|LeftMouseButton`
  (params (Key :type "Key Structure"))
  ;[1 1 1] RotateBlocks LeftMouse pressed
  (:`Pressed`
    (`/Engine/EditorBlueprintResources/StandardMacros.DoOnce` false :!label _label
      (:`Completed`
        (if (not (`self.IsRotating`))
          (`self.FnIsEnoughMana`)
          (if (`self.EnoughMana`)
            (`self.FnManaSubtractingAndReset`)
            (set `self.IsRotating` true)
            (bind _output_get (set `self.InitialBlocksRotation` (`self.K2_GetActorRotation`)))
            (bind (_direction _rotateblocksmovement) (`Timeline|Timeline` :!via `PlayFromStart`)
              (:`Update`
                (`self.K2_SetActorRotation` (`KismetMathLibrary.MakeRotator` (.roll _output_get) (.pitch _output_get) (- (.yaw _output_get) _rotateblocksmovement)))
                (`NiagaraFunctionLibrary.SpawnSystemAtLocation` null (`self.K2_GetActorLocation`)))
              (:`Finished`
                (set `self.IsRotating` false)
                (goto _label :!via `Reset`)))
            (else
              (`KismetSystemLibrary.PrintString` "Not enough mana")
              (goto _label :!via `Reset`)))
          (else
            (goto _label :!via `Reset`)))))))

(event `Key|F`
  (params (Key :type "Key Structure"))
  ;[1 1 1] RotateBlocks LeftMouse pressed
)

(event `Key|RightMouseButton`
  (params (Key :type "Key Structure"))
  ;[1 1 1] RotateBlocks RightMouse pressed
  (:`Pressed`
    (`/Engine/EditorBlueprintResources/StandardMacros.DoOnce` false :!label _label_2
      (:`Completed`
        (if (not (`self.IsRotating`))
          (`self.FnIsEnoughMana`)
          (if (`self.EnoughMana`)
            (`self.FnManaSubtractingAndReset`)
            (set `self.IsRotating` true)
            (bind _output_get (set `self.InitialBlocksRotation` (`self.K2_GetActorRotation`)))
            (bind (_direction _rotateblocksmovement) (`Timeline|Timeline_0` :!via `PlayFromStart`)
              (:`Update`
                (`self.K2_SetActorRotation` (`KismetMathLibrary.MakeRotator` (.roll _output_get) (.pitch _output_get) (- (.yaw _output_get) _rotateblocksmovement))))
              (:`Finished`
                (set `self.IsRotating` false)
                (goto _label_2 :!via `Reset`)))
            (else
              (`KismetSystemLibrary.PrintString` "Not enough mana")
              (goto _label_2 :!via `Reset`)))
          (else
            (goto _label_2 :!via `Reset`)))))))

(event `Key|E`
  (params (Key :type "Key Structure"))
  ;[1 1 1] RotateBlocks RightMouse pressed
)

(event `self.BlocksCollision.OnComponentBeginOverlap`
  (params (OverlappedComponent :type "PrimitiveComponent Object Reference") (OtherActor :type "Actor Object Reference") (OtherComp :type "PrimitiveComponent Object Reference") (OtherBodyIndex :type Integer) (bFromSweep :type Boolean) (SweepResult :type "HitResult Structure (by ref)"))
  ;[1 1 1] enable/disable rotateblocks
  (cast `/Game/Dynamic/Blueprints/CHaracterMovement/BP_PlayerCharacter` OtherActor)
  (`self.EnableInput` (`GameplayStatics.GetPlayerController` 0)))

(event `self.BlocksCollision.OnComponentEndOverlap`
  (params (OverlappedComponent :type "PrimitiveComponent Object Reference") (OtherActor :type "Actor Object Reference") (OtherComp :type "PrimitiveComponent Object Reference") (OtherBodyIndex :type Integer))
  ;[1 1 1] enable/disable rotateblocks
  (cast `/Game/Dynamic/Blueprints/CHaracterMovement/BP_PlayerCharacter` OtherActor)
  (`self.DisableInput` (`GameplayStatics.GetPlayerController` 0)))

(fn `FnIsEnoughMana`
  (bind _asbp_player_character (cast `/Game/Dynamic/Blueprints/CHaracterMovement/BP_PlayerCharacter` (`GameplayStatics.GetPlayerCharacter` 0)))
  (if (>= (- (`/Game/Dynamic/Blueprints/CHaracterMovement/BP_PlayerCharacter.ManaPoints` _asbp_player_character) (`self.ManaCostToRotate`)) 0)
    (set `self.EnoughMana` true))
  (return))

(fn `FnManaSubtractingAndReset`
  (bind _asbp_player_character (cast `/Game/Dynamic/Blueprints/CHaracterMovement/BP_PlayerCharacter` (`GameplayStatics.GetPlayerCharacter` 0)))
  (set `/Game/Dynamic/Blueprints/CHaracterMovement/BP_PlayerCharacter.ManaPoints` (- (`/Game/Dynamic/Blueprints/CHaracterMovement/BP_PlayerCharacter.ManaPoints` _asbp_player_character) (`self.ManaCostToRotate`)) _asbp_player_character)
  (set `self.EnoughMana` false)
  (return))

(fn `GetInteractionWidgetRef`
  (returns (Ref :type "WidgetComponent Object Reference"))
  (return (`self.Widget`)))

(fn `OnRep_InteractToggle`
  ;[1 1 1] Visibility of Point light
)

(fn `UserConstructionScript`)