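; BP_KeyStone is an interactable stone that the player can move once they have collected two keys.
; Overlapping StoneCollision sets the player's prompt message and enables UseObject input if the key count matches; leaving clears both.
; UseObject plays a timeline that drives the stone's relative Z location.
; A separate actor-level overlap increments the player's KeyStonePushed counter on every overlap, regardless of keys.
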(event `InputAction|UseObject`
  (params (Key :type "Key Structure"))
  (:`Pressed`
    (bind (_direction _stonemovement2) (`Timeline|StoneMoved`)
      (:`Update`
        (`SceneComponent.K2_SetRelativeLocation` (`self.KeyStone`) (`KismetMathLibrary.MakeVector` 0.0 0.0 (* _stonemovement2 30.0)) false false)))))

(event `self.StoneCollision.OnComponentBeginOverlap`
  (params (OverlappedComponent :type "PrimitiveComponent Object Reference") (OtherActor :type "Actor Object Reference") (OtherComp :type "PrimitiveComponent Object Reference") (OtherBodyIndex :type Integer) (bFromSweep :type Boolean) (SweepResult :type "HitResult Structure (by ref)"))
  (bind _asbp_player_character (cast `/Game/Dynamic/Blueprints/CHaracterMovement/BP_PlayerCharacter` OtherActor))
  (if (== (`/Game/Dynamic/Blueprints/CHaracterMovement/BP_PlayerCharacter.KeysCollected` _asbp_player_character) 2)
    (set `/Game/Dynamic/Blueprints/CHaracterMovement/BP_PlayerCharacter.ScreenMessage` "Press F to move stone" _asbp_player_character)
    (`self.EnableInput` (`GameplayStatics.GetPlayerController` 0))
    (else
      (set `/Game/Dynamic/Blueprints/CHaracterMovement/BP_PlayerCharacter.ScreenMessage` "You must collect all keys to move this stone" _asbp_player_character))))

(event `self.StoneCollision.OnComponentEndOverlap`
  (params (OverlappedComponent :type "PrimitiveComponent Object Reference") (OtherActor :type "Actor Object Reference") (OtherComp :type "PrimitiveComponent Object Reference") (OtherBodyIndex :type Integer))
  (bind _asbp_player_character (cast `/Game/Dynamic/Blueprints/CHaracterMovement/BP_PlayerCharacter` OtherActor))
  (set `/Game/Dynamic/Blueprints/CHaracterMovement/BP_PlayerCharacter.ScreenMessage` "" _asbp_player_character)
  (`self.DisableInput` (`GameplayStatics.GetPlayerController` 0)))

(event `self.ReceiveActorBeginOverlap`
  (params (OtherActor :type "Actor Object Reference"))
  (bind _asbp_player_character (cast `/Game/Dynamic/Blueprints/CHaracterMovement/BP_PlayerCharacter` OtherActor))
  (set `/Game/Dynamic/Blueprints/CHaracterMovement/BP_PlayerCharacter.KeyStonePushed` (+ (`/Game/Dynamic/Blueprints/CHaracterMovement/BP_PlayerCharacter.KeyStonePushed` _asbp_player_character) 1) _asbp_player_character))

(fn `UserConstructionScript`)